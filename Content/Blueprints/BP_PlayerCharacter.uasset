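; BP_PlayerCharacter is the player character Blueprint that manages the local player's crosshair and capture point progress UI.
; On BeginPlay it adds the crosshair widget for the locally controlled player.
; Capture point overlap notifications store or clear the point and add or remove a progress bar widget.
; While overlapping, Tick finds the bar through GetAllWidgetsOfClass and sets it from the point's capture percentage.
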(event EventBeginPlay
  ;[1 1 1] Create the crosshair UI
  (if (Pawn|IsLocallyControlled)
    (bind _returnvalue (UserInterface|CreateWidget "/Game/UI/WBP_Crosshair.WBP_Crosshair_C"))
    (UserInterface|Viewport|AddtoViewport _returnvalue 0)))

(event EventTick
  (params (DeltaSeconds :type Float%20%28single-precision%29))
  ;[1 1 1] Update the capture progress bar if we're overlapping a capture point
  (if (Variables|Default|GetbOverlappingCapturePoint)
    (bind _foundwidgets (Widget|GetAllWidgetsOfClass "/Game/UI/WBP_CaptureProgressBar.WBP_CaptureProgressBar_C" true))
    (for _array_element _foundwidgets
      (Variables|/Game/UI/WBP_CaptureProgressBar.WBP_CaptureProgressBar_C|SetProgress _array_element (/ (Variables|/Script/CaptureGame.CGCapturePoint|GetCurrentCapturePercentage (Variables|Default|GetOverlappedCapturePoint)) 1e+02)))))

(event EventNotifyBeginOverlapCapturePoint
  (params (CapturePoint :type CG%20Capture%20Point%20Object%20Reference))
  ;[1 1 1] Create 'Capture Progress' bar
  (if (Pawn|IsLocallyControlled)
    (Variables|Default|SetbOverlappingCapturePoint true)
    (Variables|Default|SetOverlappedCapturePoint CapturePoint)
    (bind _returnvalue (UserInterface|CreateWidget "/Game/UI/WBP_CaptureProgressBar.WBP_CaptureProgressBar_C"))
    (UserInterface|Viewport|AddtoViewport _returnvalue 0)))

(event EventNotifyEndOverlapCapturePoint
  (params (CapturePoint :type CG%20Capture%20Point%20Object%20Reference))
  ;[1 1 1] Remove 'Capture Progress' bar
  (if (Pawn|IsLocallyControlled)
    (Variables|Default|SetbOverlappingCapturePoint false)
    (Variables|Default|SetOverlappedCapturePoint 0)
    (bind _foundwidgets (Widget|GetAllWidgetsOfClass "/Game/UI/WBP_CaptureProgressBar.WBP_CaptureProgressBar_C" true))
    (Widget|RemovefromParent _foundwidgets)))

(fn ConstructionScript)