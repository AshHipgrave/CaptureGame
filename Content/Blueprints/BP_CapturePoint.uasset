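; Capture point actor that shows a capture progress bar on screen while something overlaps it.
; Any actor beginning overlap adds a new WBP_CaptureProgressBar to the viewport, and any end overlap removes all such top-level widgets.
; Tick finds every such widget by class and sets its progress from CurrentCapturePercentage, which this graph only reads.
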(event EventBeginPlay)

(event Collision|EventActorBeginOverlap
  (params (OtherActor :type Actor%20Object%20Reference))
  ;[1 1 1] Create the 'Capture Progress' bar when players overlap
  (bind _returnvalue (UserInterface|CreateWidget "/Game/UI/WBP_CaptureProgressBar.WBP_CaptureProgressBar_C"))
  (UserInterface|Viewport|AddtoViewport _returnvalue 0))

(event EventTick
  (params (DeltaSeconds :type Float%20%28single-precision%29))
  (bind _foundwidgets (Widget|GetAllWidgetsOfClass "/Game/UI/WBP_CaptureProgressBar.WBP_CaptureProgressBar_C" true))
  (for _array_element _foundwidgets
    (Variables|/Game/UI/WBP_CaptureProgressBar.WBP_CaptureProgressBar_C|SetProgress _array_element (/ (Variables|Default|GetCurrentCapturePercentage) 1e+02))))

(event Collision|EventActorEndOverlap
  (params (OtherActor :type Actor%20Object%20Reference))
  ;[1 1 1] Remove the 'Capture Progress' bar when players no longer overlap
  (bind _foundwidgets (Widget|GetAllWidgetsOfClass "/Game/UI/WBP_CaptureProgressBar.WBP_CaptureProgressBar_C" true))
  (Widget|RemovefromParent _foundwidgets))

(fn ConstructionScript)